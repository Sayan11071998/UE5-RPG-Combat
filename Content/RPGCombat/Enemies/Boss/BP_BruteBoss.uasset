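; BP_BruteBoss is a Brute boss enemy that handles its death sequence and an on-screen nameplate.
; The EnemyDeath event plays a death montage, then destroys the actor after a short delay.
; When an RPG character enters NamePlateSphere, it creates a boss nameplate widget, passes itself to it and adds it to the viewport.
; Leaving the sphere removes that widget.
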(event OnComponentBeginOverlap(NamePlateSphere)
  (params (OverlappedComponent :type Primitive%20Component%20Object%20Reference) (OtherActor :type Actor%20Object%20Reference) (OtherComp :type Primitive%20Component%20Object%20Reference) (OtherBodyIndex :type Integer) (bFromSweep :type Boolean) (SweepResult :type Hit%20Result%20Structure%20%28by%20ref%29))
  ;[0 0 0 0.5] Boss Nameplate
  (Utilities|Casting|CastToBP_RPGCharacter OtherActor)
  (bind _returnvalue (UserInterface|CreateWidget "/Game/RPGCombat/UI/WBP_BruteBossNP.WBP_BruteBossNP_C"))
  (bind _output_get (Variables|Default|SetBruteBossNP _returnvalue))
  (Variables|/Game/RPGCombat/UI/WBP_BruteBossNP.WBP_BruteBossNP_C|SetBoss _output_get self)
  (UserInterface|Viewport|AddtoViewport _output_get 0))

(event OnComponentEndOverlap(NamePlateSphere)
  (params (OverlappedComponent :type Primitive%20Component%20Object%20Reference) (OtherActor :type Actor%20Object%20Reference) (OtherComp :type Primitive%20Component%20Object%20Reference) (OtherBodyIndex :type Integer))
  ;[0 0 0 0.5] Boss Nameplate
  (Utilities|Casting|CastToBP_RPGCharacter OtherActor)
  (Widget|RemovefromParent (Variables|Default|GetBruteBossNP)))

(event EventEnemyDeath
  ;[0 0 0 0.5] Enemy Death
  (Animation|PlayAnimMontage "/Game/RPGCombat/Enemies/Brute/Montages/AM_BruteDeathMontage.AM_BruteDeathMontage" 1.0 "None")
  (Utilities|FlowControl|Delay 2.1)
  (Actor|DestroyActor))

(fn ConstructionScript)
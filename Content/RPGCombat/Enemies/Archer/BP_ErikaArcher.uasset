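; BP_ErikaArcher is the Erika archer enemy Blueprint, whose logic here drives a floating nameplate that appears when the player is nearby.
; On BeginPlay it passes itself to the WBP_ErikaNP widget on the Nameplate component and hides it.
; NameplateSphere overlaps with a BP_RPGCharacter show the widget on entry and hide it on exit, reassigning the enemy reference each time.
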(event OnComponentBeginOverlap(NameplateSphere)
  (params (OverlappedComponent :type Primitive%20Component%20Object%20Reference) (OtherActor :type Actor%20Object%20Reference) (OtherComp :type Primitive%20Component%20Object%20Reference) (OtherBodyIndex :type Integer) (bFromSweep :type Boolean) (SweepResult :type Hit%20Result%20Structure%20%28by%20ref%29))
  (bind _nameplate (Variables|Default|GetNameplate))
  (bind _returnvalue (UserInterface|GetUserWidgetObject _nameplate))
  ;[0 0 0 0.5] Enemy Nameplate
  (Utilities|Casting|CastToBP_RPGCharacter OtherActor)
  (bind _aswbp_erika_np (Utilities|Casting|CastToWBP_ErikaNP _returnvalue))
  (Variables|/Game/RPGCombat/UI/WBP_ErikaNP.WBP_ErikaNP_C|SetEnemy _aswbp_erika_np self)
  (Widget|SetVisibility _returnvalue "Visible"))

(event OnComponentEndOverlap(NameplateSphere)
  (params (OverlappedComponent :type Primitive%20Component%20Object%20Reference) (OtherActor :type Actor%20Object%20Reference) (OtherComp :type Primitive%20Component%20Object%20Reference) (OtherBodyIndex :type Integer))
  (bind _nameplate (Variables|Default|GetNameplate))
  (bind _returnvalue (UserInterface|GetUserWidgetObject _nameplate))
  ;[0 0 0 0.5] Enemy Nameplate
  (Utilities|Casting|CastToBP_RPGCharacter OtherActor)
  (bind _aswbp_erika_np (Utilities|Casting|CastToWBP_ErikaNP _returnvalue))
  (Variables|/Game/RPGCombat/UI/WBP_ErikaNP.WBP_ErikaNP_C|SetEnemy _aswbp_erika_np self)
  (Widget|SetVisibility _returnvalue "Hidden"))

(event EventBeginPlay
  (bind _nameplate (Variables|Default|GetNameplate))
  (bind _returnvalue (UserInterface|GetUserWidgetObject _nameplate))
  ;[0 0 0 0.5] Enemy Nameplate
  (bind _aswbp_erika_np (Utilities|Casting|CastToWBP_ErikaNP _returnvalue))
  (Variables|/Game/RPGCombat/UI/WBP_ErikaNP.WBP_ErikaNP_C|SetEnemy _aswbp_erika_np self)
  (Widget|SetVisibility _returnvalue "Hidden"))

(fn ConstructionScript)
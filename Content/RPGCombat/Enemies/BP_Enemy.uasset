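; BP_Enemy is the enemy actor for the RPG combat game, with a proximity-based nameplate and a death sequence.
; On begin play it links the WBP_BruteNP widget to itself and hides it.
; The NamePlateSphere overlap shows the nameplate when a BP_RPGCharacter enters and hides it on exit.
; EnemyDeath plays the Brute death montage, waits briefly, then destroys the actor.
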(event OnComponentBeginOverlap(NamePlateSphere)
  (params (OverlappedComponent :type Primitive%20Component%20Object%20Reference) (OtherActor :type Actor%20Object%20Reference) (OtherComp :type Primitive%20Component%20Object%20Reference) (OtherBodyIndex :type Integer) (bFromSweep :type Boolean) (SweepResult :type Hit%20Result%20Structure%20%28by%20ref%29))
  (bind _nameplate (Variables|Default|GetNamePlate))
  (bind _returnvalue (UserInterface|GetUserWidgetObject _nameplate))
  ;[0 0 0 0.5] Enemy Nameplate
  (Utilities|Casting|CastToBP_RPGCharacter OtherActor)
  (bind _aswbp_brute_np (Utilities|Casting|CastToWBP_BruteNP _returnvalue))
  (Variables|/Game/RPGCombat/UI/WBP_BruteNP.WBP_BruteNP_C|SetEnemy _aswbp_brute_np self)
  (Widget|SetVisibility _returnvalue "Visible"))

(event OnComponentEndOverlap(NamePlateSphere)
  (params (OverlappedComponent :type Primitive%20Component%20Object%20Reference) (OtherActor :type Actor%20Object%20Reference) (OtherComp :type Primitive%20Component%20Object%20Reference) (OtherBodyIndex :type Integer))
  (bind _nameplate (Variables|Default|GetNamePlate))
  (bind _returnvalue (UserInterface|GetUserWidgetObject _nameplate))
  ;[0 0 0 0.5] Enemy Nameplate
  (Utilities|Casting|CastToBP_RPGCharacter OtherActor)
  (bind _aswbp_brute_np (Utilities|Casting|CastToWBP_BruteNP _returnvalue))
  (Variables|/Game/RPGCombat/UI/WBP_BruteNP.WBP_BruteNP_C|SetEnemy _aswbp_brute_np self)
  (Widget|SetVisibility _returnvalue "Hidden"))

(event EventEnemyDeath
  ;[0 0 0 0.5] Enemy Death
  (Animation|PlayAnimMontage "/Game/RPGCombat/Enemies/Montages/AM_BruteDeathMontage.AM_BruteDeathMontage" 1.0 "None")
  (Utilities|FlowControl|Delay 2.1)
  (Actor|DestroyActor))

(event EventBeginPlay
  (bind _nameplate (Variables|Default|GetNamePlate))
  (bind _returnvalue (UserInterface|GetUserWidgetObject _nameplate))
  ;[0 0 0 0.5] Enemy Nameplate
  (bind _aswbp_brute_np (Utilities|Casting|CastToWBP_BruteNP _returnvalue))
  (Variables|/Game/RPGCombat/UI/WBP_BruteNP.WBP_BruteNP_C|SetEnemy _aswbp_brute_np self)
  (Widget|SetVisibility _returnvalue "Hidden"))

(fn ConstructionScript)